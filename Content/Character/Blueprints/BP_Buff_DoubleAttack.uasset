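; BP_Buff_DoubleAttack is a buff pickup that triggers DoubleAttack on the ThirdPersonCharacter that overlaps it.
; The overlap is handled only on the authority, which applies the buff and then destroys the actor.
; A Name widget component displays "攻击UP" (Attack UP), set at BeginPlay.
; Each tick the label's yaw follows the first player controller's control rotation plus 180 degrees to face the camera.
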(event EventBeginPlay
  (bind _asbuff (Utilities|Casting|CastToBuff (UserInterface|GetWidget (Variables|Default|GetName))))
  (Default|SetName _asbuff "攻击UP"))

(event Collision|EventActorBeginOverlap
  (params (OtherActor :type Actor%20Object%20Reference))
  (Networking|SwitchHasAuthority
    (:Authority
      (bind _asthird_person_character (Utilities|Casting|CastToThirdPersonCharacter OtherActor))
      (Default|DoubleAttack _asthird_person_character)
      (Actor|DestroyActor))))

(event EventTick
  (params (DeltaSeconds :type Float%20%28single-precision%29))
  (CallFunction|HPWidgetLookatCamera))

(fn ConstructionScript)

(fn HPWidgetLookatCamera
  (bind _name (Variables|Default|GetName))
  (bind _returnvalue (Transformation|GetWorldRotation _name))
  (Transformation|SetWorldRotation _name (Math|Rotator|MakeRotator (.roll _returnvalue) (.pitch _returnvalue) (+ (.Yaw (Math|Rotator|BreakRotator (Pawn|GetControlRotation (Game|GetPlayerController 0) :!class /Script/Engine.Controller))) 1.8e+02)) false false))