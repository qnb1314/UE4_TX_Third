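; Monster AI controller Blueprint that runs the AI_Behavier behavior tree when it possesses a pawn.
; It exposes three setter functions that write the target actor, line-of-sight flag and death flag to Blackboard keys held in name variables.
; The file contains no perception or decision logic, and its Tick event is empty.
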(event EventTick
  (params (DeltaSeconds :type Float%20%28single-precision%29)))

(event EventPossess
  (params (PossessedPawn :type Pawn%20Object%20Reference))
  (AI|RunBehaviorTree "/Game/Monster/AI/AI_Behavier.AI_Behavier"))

(fn ConstructionScript)

(fn UpdateTargetActor
  (params (Target_Actor :type Actor%20Object%20Reference))
  (AI|Components|Blackboard|SetValueasObject (Variables|Default|GetBlackboard) (Variables|Keyname|GetTarget_Actor_Name) Target_Actor))

(fn UpdateHasLineOfSight
  (params (HasLineOfSight :type Boolean))
  (AI|Components|Blackboard|SetValueasBool (Variables|Default|GetBlackboard) (Variables|Keyname|GetHasLineOfSight_Name) HasLineOfSight))

(fn UpdateDeath
  (params (Ifdeath :type Boolean))
  (AI|Components|Blackboard|SetValueasBool (Variables|Default|GetBlackboard) (Variables|KeyName|GetIsDeath) Ifdeath))